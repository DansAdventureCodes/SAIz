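; BP_WoodenBox is a box that the top-down character can pick up by pressing Space while near it.
; Overlap events on PickupCollision store the overlapping BP_TopDownCharacter as a reference and clear it when that character leaves.
; On Space, a valid reference triggers a debug print and a snapped, welded attach to the character's HoldPosition, with no detach logic.
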(event `self.PickupCollision.OnComponentBeginOverlap`
  (params (OverlappedComponent :type "PrimitiveComponent Object Reference") (OtherActor :type "Actor Object Reference") (OtherComp :type "PrimitiveComponent Object Reference") (OtherBodyIndex :type Integer) (bFromSweep :type Boolean) (SweepResult :type "HitResult Structure (by ref)"))
  (bind _asbp_top_down_character (cast `/Game/TopDown/Blueprints/BP_TopDownCharacter` (stale `self.PickupCollision.OnComponentEndOverlap` OtherActor)))
  (set `self.CharacterRef` _asbp_top_down_character))

(event `self.PickupCollision.OnComponentEndOverlap`
  (params (OverlappedComponent :type "PrimitiveComponent Object Reference") (OtherActor :type "Actor Object Reference") (OtherComp :type "PrimitiveComponent Object Reference") (OtherBodyIndex :type Integer))
  (cast `/Game/TopDown/Blueprints/BP_TopDownCharacter` OtherActor)
  (set `self.CharacterRef` null))

(event `Key|SpaceBar`
  (params (Key :type "Key Structure"))
  (bind _characterref (`self.CharacterRef`))
  (:`Pressed`
    (if (`KismetSystemLibrary.IsValid` _characterref)
      (`KismetSystemLibrary.PrintString` "Attached")
      (`self.K2_AttachToComponent` (`/Game/TopDown/Blueprints/BP_TopDownCharacter.HoldPosition` _characterref) "None" "SnapToTarget" "SnapToTarget" "SnapToTarget" true))))

(fn `UserConstructionScript`)